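; Enemy melee attack gameplay ability that turns the avatar toward its combat target and plays a random tagged attack montage.
; The montage's gameplay event triggers a small radius check at that montage's combat socket.
; Non-friendly live players found there take damage and get a blood effect call, and any hit fires one MeleeImpact gameplay cue.
; The ability ends after the hit check or when the montage completes, is interrupted or is cancelled.
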(event Ability|EventActivateAbility
  (bind _returnvalue (Ability|GetAvatarActorfromActorInfo))
  (Variables|Default|SetHasHitTarget? false)
  (bind _returnvalue_2 (Class|EnemyInterface|GetCombatTarget(Message) _returnvalue))
  (bind _ascombat_interface (Utilities|Casting|CastToCombatInterface _returnvalue))
  (Class|CombatInterface|UpdateFacingTarget _ascombat_interface (Transformation|GetActorLocation _returnvalue_2))
  (bind _returnvalue_3 (Class|CombatInterface|GetAttackMontages(Message) (Ability|GetAvatarActorfromActorInfo)))
  (bind _output_get (Variables|Default|SetTaggedMontage (Class|AuraDamageGameplayAbility|GetRandomTaggedMontage _returnvalue_3)))
  (|PlayMontageandWaitProxy "None" (.Montage (Utilities|Struct|BreakTaggedMontage _output_get)) 1.0 "None" false 1.0 0.0
    (:then
      (Ability|Tasks|WaitGameplayEvent (.MontageTag (Utilities|Struct|BreakTaggedMontage _output_get)) 0
        (:EventReceived
          (bind _returnvalue_4 (Class|CombatInterface|GetCombatSocketLocation(Message) (Ability|GetAvatarActorfromActorInfo) (.SocketTag (Utilities|Struct|BreakTaggedMontage _output_get))))
          (Variables|Default|SetCombatSocketLocation _returnvalue_4)
          (bind _outoverlappingactors (Class|AuraAbilitySystemLibrary|GetLivePlayersWithinRadius self (Utilities|Array|MakeArray (Ability|GetAvatarActorfromActorInfo)) 45.0 (Variables|Default|GetCombatSocketLocation)))
          (for _array_element _outoverlappingactors
            (if (Class|AuraAbilitySystemLibrary|IsNotFriend _array_element (Ability|GetAvatarActorfromActorInfo))
              (Class|AuraDamageGameplayAbility|CauseDamage _array_element)
              (Variables|Default|SetHasHitTarget? true)
              (Class|CombatInterface|GetBloodEffect(Message) _array_element)))
          (if (Variables|Default|GetHasHitTarget?)
            (bind _returnvalue_5 (Class|EnemyInterface|GetCombatTarget(Message) (Ability|GetAvatarActorfromActorInfo)))
            (Class|GameplayAbility|ExecuteGameplayCuewithParams "(TagName=\"GameplayCue.MeleeImpact\")" (Ability|GameplayCue|MakeGameplayCueParameters :AggregatedSourceTags (GameplayTags|MakeGameplayTagContainerfromTag (.montagetag (Variables|Default|GetTaggedMontage))) :Location (Variables|Default|GetCombatSocketLocation) :EffectCauser (Ability|GetAvatarActorfromActorInfo) :SourceObject _returnvalue_5)))
          (Ability|EndAbility))))
    (:OnCompleted
      (Ability|EndAbility :!label _label))
    (:OnInterrupted
      (goto _label))
    (:OnCancelled
      (goto _label))))

(event Ability|EventOnEndAbility
  (params (bWasCancelled :type Boolean)))