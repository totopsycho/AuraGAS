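; BP_FadeActor is an actor whose mesh fades out and back in through FadeOut and Fadein events.
; Construction caches the original materials and creates dynamic instances from FadeMaterialInstances.
; FadeOut swaps in those instances and plays a timeline driving their "Fade" parameter, while Fadein reverses it.
; When the timeline finishes, a high value restores original materials; BlockVisibility optionally toggles Visibility collision between Block and Ignore.
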(event EventBeginPlay)

(event Collision|EventActorBeginOverlap
  (params (OtherActor :type Actor%20Object%20Reference)))

(event EventTick
  (params (DeltaSeconds :type Float%20%28single-precision%29)))

(event EventFadeOut
  (CallFunction|SetMaterialstoDynamicInstance)
  (bind _fade (Timeline|FadeTimeLine Play)
    (:Update
      (for _array_element (Variables|Default|GetDynamicMatInst)
        (Rendering|Material|SetScalarParameterValue _array_element "Fade" _fade :!class /Script/Engine.MaterialInstanceDynamic)))
    (:Finished
      (if (>= _fade 1.0)
        (CallFunction|ResetMaterials)
        (if (Variables|Default|GetBlockVisibility)
          (Collision|SetCollisionResponsetoChannel (Variables|Default|GetMesh) "ECC_Visibility" "ECR_Block"))
        (elif (<= _fade 0.0)
          (if (Variables|Default|GetBlockVisibility)
            (Collision|SetCollisionResponsetoChannel (Variables|Default|GetMesh) "ECC_Visibility" "ECR_Ignore")))))))

(event EventFadein
  (bind _fade (Timeline|FadeTimeLine Reverse)
    (:Update
      (for _array_element (Variables|Default|GetDynamicMatInst)
        (Rendering|Material|SetScalarParameterValue _array_element "Fade" _fade :!class /Script/Engine.MaterialInstanceDynamic)))
    (:Finished
      (if (>= _fade 1.0)
        (CallFunction|ResetMaterials)
        (if (Variables|Default|GetBlockVisibility)
          (Collision|SetCollisionResponsetoChannel (Variables|Default|GetMesh) "ECC_Visibility" "ECR_Block"))
        (elif (<= _fade 0.0)
          (if (Variables|Default|GetBlockVisibility)
            (Collision|SetCollisionResponsetoChannel (Variables|Default|GetMesh) "ECC_Visibility" "ECR_Ignore")))))))

(fn ConstructionScript
  (Utilities|Array|Clear (Variables|Default|GetDynamicMatInst))
  (Variables|Default|SetOriginalMaterials (Rendering|Material|GetMaterials (Variables|Default|GetMesh)))
  (for _array_element (Variables|Default|GetFadeMaterialInstances)
    (bind _returnvalue (Rendering|Material|CreateDynamicMaterialInstance _array_element "None" "None" :!class /Script/Engine.KismetMaterialLibrary))
    (Utilities|Array|AddUnique (Variables|Default|GetDynamicMatInst) _returnvalue)))

(fn SetMaterialstoDynamicInstance
  (for (_array_element _array_index) (Variables|Default|GetDynamicMatInst)
    (Rendering|Material|SetMaterial (Variables|Default|GetMesh) _array_index _array_element)))

(fn ResetMaterials
  (for (_array_element _array_index) (Variables|Default|GetOriginalMaterials)
    (Rendering|Material|SetMaterial (Variables|Default|GetMesh) _array_index _array_element)))